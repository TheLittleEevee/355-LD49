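; NPC Blueprint with a configurable Paper2D flipbook sprite and up to three lines of dialogue.
; The construction script applies the Sprite to the flipbook component when valid.
; GiveTextInfo sends the Name and current line to the dialogue widget, then overwrites Speech1 with the next line for the following call.
; A "null" string marks unused lines, and dialogue stays on the last available one.
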(fn ConstructionScript
  (Utilities|IsValid (Variables|Default|GetSprite)
    (:Is%20Valid
      (Sprite|SetFlipbook (Variables|Default|GetPaperFlipbook) (Variables|Default|GetSprite)))))

(fn GiveTextInfo
  (params (Dialogue%20Widget :type Dialogue%20Object%20Reference) (Player :type The%20Player%20Object%20Reference))
  (Default|SetText Dialogue%20Widget (Variables|Default|GetName) (Variables|Default|GetSpeech%201))
  (if (Utilities|Enum|NotEqual(Enum) (Variables|Default|GetSpeech%202) "null")
    (if (or (Utilities|Enum|Equal(Enum) (Variables|Default|GetSpeech%201) (Variables|Default|GetSpeech%202)) (Utilities|Enum|Equal(Enum) (Variables|Default|GetSpeech%201) (Variables|Default|GetSpeech%203)))
      (if (Utilities|Enum|NotEqual(Enum) (Variables|Default|GetSpeech%203) "null")
        (Variables|Default|SetSpeech%201 (Variables|Default|GetSpeech%203)))
      (else
        (Variables|Default|SetSpeech%201 (Variables|Default|GetSpeech%202))))))