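; Child NPC Blueprint that supplies dialogue and changes appearance once the player has cured the child.
; GiveTextInfo checks the ChildisCured flag in the player's Details and sends the child's name and one of two speeches to the dialogue widget.
; When cured, it also swaps the Paper2D flipbook to the healthy boy and calls FinishedHelping on the player.
; The construction script only calls its parent.
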(event EventGiveTextInfo
  (params (Dialogue%20Widget :type Dialogue%20Object%20Reference) (Player :type The%20Player%20Object%20Reference))
  (if (.childiscured (Variables|/Game/Blueprints/PlayerAndGame/ThePlayer.ThePlayer_C|GetDetails Player))
    (Sprite|SetFlipbook (Variables|Default|GetPaperFlipbook) "/Game/Art/Assets/Characters/healthy_boy_Flipbook.healthy_boy_Flipbook")
    (Default|SetText Dialogue%20Widget (Variables|Default|GetName) (Variables|Default|GetSpeech%202))
    (Default|FinishedHelping Player "Child")
    (else
      (Default|SetText Dialogue%20Widget (Variables|Default|GetName) (Variables|Default|GetSpeech%201)))))

(fn ConstructionScript
  (|CallParentFunction))