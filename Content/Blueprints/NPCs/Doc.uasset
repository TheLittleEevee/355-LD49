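; Doc NPC, a Paper2D cleric who joins the player in a quest to heal a child.
; Dialogue shows generic villager text until the player has talked to the parent, then starts following and varies by quest state.
; While following, Tick places Doc just ahead of the player at fixed height, choosing walk flipbooks from player facing and input.
; DocatDestination stops following, sets the standing flipbook and calls the player's ChildIsBetter.
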(event Custom|Doc%20at%20Destination
  (Variables|Default|SetIs%20Following false)
  (Sprite|SetFlipbook (Variables|Default|GetPaperFlipbook) "/Game/Art/Assets/Characters/cleric/front/cleric_standing.cleric_standing")
  (Default|ChildIsBetter (stale EventGiveTextInfo Player)))

(event EventGiveTextInfo
  (params (Dialogue%20Widget :type Dialogue%20Object%20Reference) (Player :type The%20Player%20Object%20Reference))
  (bind _name (Variables|Default|GetName))
  (if (.talkedtoparent (Variables|/Game/Blueprints/PlayerAndGame/ThePlayer.ThePlayer_C|GetDetails Player))
    (if (Variables|Default|GetHas%20Talked%20To?)
      (if (Variables|Default|GetIs%20Following)
        (Default|SetText Dialogue%20Widget _name (Variables|Default|GetSpeech%202))
        (else
          (Default|SetText Dialogue%20Widget _name (Variables|Default|GetSpeech%203))))
      (else
        (Variables|Default|SetHas%20Talked%20To? true)
        (Default|SetText Dialogue%20Widget _name (Variables|Default|GetSpeech%201))
        (Variables|Default|SetIs%20Following true)))
    (else
      (Default|SetText Dialogue%20Widget "Villager" "What a great party!"))))

(event EventTick
  (params (DeltaSeconds :type Float%20%28single-precision%29))
  (if (Variables|Default|GetIs%20Following)
    (CallFunction|DocFollowing (stale EventGiveTextInfo Player))))

(fn ConstructionScript
  (|CallParentFunction))

(fn DocFollowing
  (params (Player :type The%20Player%20Object%20Reference))
  (bind _returnvalue (Transformation|GetActorForwardVector Player))
  (bind _returnvalue_2 (Transformation|GetActorLocation Player))
  (bind _paperflipbook (Variables|Default|GetPaperFlipbook))
  (bind _returnvalue_3 (+ _returnvalue_2 _returnvalue))
  (bind _returnvalue_4 (Math|Interpolation|VInterpTo _returnvalue_2 _returnvalue_3 0.5 1e+02))
  (Transformation|SetActorLocation (Math|Vector|MakeVector (.x _returnvalue_4) (.y _returnvalue_4) (.z (Transformation|GetActorLocation))) true false)
  (Variables|Default|SetDirection%20Facing (Variables|/Game/Blueprints/PlayerAndGame/ThePlayer.ThePlayer_C|GetFacing Player))
  (if (== (Variables|/Game/Blueprints/PlayerAndGame/ThePlayer.ThePlayer_C|GetRight%20Axis Player) 0.0)
    (if (Utilities|Enum|Equal(Enum) (Variables|Default|GetDirection%20Facing) "F")
      (Sprite|SetFlipbook _paperflipbook "/Game/Art/Assets/Characters/cleric/back/cleric_walk_back.cleric_walk_back")
      (elif (Utilities|Enum|Equal(Enum) (Variables|Default|GetDirection%20Facing) "B")
        (Sprite|SetFlipbook _paperflipbook "/Game/Art/Assets/Characters/cleric/front/cleric_walk_front.cleric_walk_front")))
    (elif (Utilities|Enum|Equal(Enum) (Variables|Default|GetDirection%20Facing) "R")
      (Sprite|SetFlipbook _paperflipbook "/Game/Art/Assets/Characters/cleric/right/cleric_walk_right.cleric_walk_right")
      (elif (Utilities|Enum|Equal(Enum) (Variables|Default|GetDirection%20Facing) "L")
        (Sprite|SetFlipbook _paperflipbook "/Game/Art/Assets/Characters/cleric/left/cleric_walk_left.cleric_walk_left")))))