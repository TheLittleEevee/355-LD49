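; Bard NPC that gives the player dialogue for a music sheet collection quest.
; GiveTextInfo shows the first speech on the initial talk and on later talks until the game instance's PlayerDetails holds exactly three music sheets.
; It then shows the second speech and tells the player it has finished helping the Bard.
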(event EventGiveTextInfo
  (params (Dialogue%20Widget :type Dialogue%20Object%20Reference) (Player :type The%20Player%20Object%20Reference))
  (bind _name (Variables|Default|GetName))
  (if (Variables|Default|GetHas%20Talked%20To?)
    (bind _asmy_game_instance (Utilities|Casting|CastToMyGameInstance (Game|GetGameInstance)))
    (bind _output_get (Variables|Default|SetPlayer's%20Details (Variables|/Game/Blueprints/MyGameInstance.MyGameInstance_C|GetPlayer%20Details _asmy_game_instance)))
    (if (== (.musicsheets _output_get) 3)
      (Default|SetText Dialogue%20Widget _name (Variables|Default|GetSpeech%202))
      (Default|FinishedHelping Player "Bard")
      (else
        (Default|SetText Dialogue%20Widget _name (Variables|Default|GetSpeech%201) :!label _label)))
    (else
      (Variables|Default|SetHas%20Talked%20To? true)
      (goto _label))))

(fn ConstructionScript
  (|CallParentFunction))