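; Parent NPC, shown with a Paper2D flipbook, that gives the player dialogue about a sick child.
; GiveTextInfo fills the dialogue widget with the first speech, marks the parent as talked to and notifies the player through TalkedToParent.
; Once talked to, if the player's details show the child is cured, it switches to the happy mom flipbook and shows the second speech.
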(event EventGiveTextInfo
  (params (Dialogue%20Widget :type Dialogue%20Object%20Reference) (Player :type The%20Player%20Object%20Reference))
  (if (Variables|Default|GetHas%20Talked%20to?)
    (if (.childiscured (Variables|/Game/Blueprints/PlayerAndGame/ThePlayer.ThePlayer_C|GetDetails Player))
      (Sprite|SetFlipbook (Variables|Default|GetPaperFlipbook) "/Game/Art/Assets/Characters/happy_mom_Flipbook.happy_mom_Flipbook")
      (Default|SetText Dialogue%20Widget (Variables|Default|GetName) (Variables|Default|GetSpeech%202))
      (else
        (Default|SetText Dialogue%20Widget (Variables|Default|GetName) (Variables|Default|GetSpeech%201) :!label _label)
        (Variables|Default|SetHas%20Talked%20to? true)
        (Default|TalkedtoParent Player)))
    (else
      (goto _label))))

(fn ConstructionScript
  (|CallParentFunction))