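; Destination is a trigger-box Blueprint that marks an arrival point for the Mage, the Doc or the player.
; On box overlap, the WhosItFor value selects which class the overlapping actor is cast to, ignoring actors that fail the cast.
; The Mage and Doc are notified that they reached their destination, while any other value makes the player run its finish check.
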(event OnComponentBeginOverlap(Box)
  (params (OverlappedComponent :type Primitive%20Component%20Object%20Reference) (OtherActor :type Actor%20Object%20Reference) (OtherComp :type Primitive%20Component%20Object%20Reference) (OtherBodyIndex :type Integer) (bFromSweep :type Boolean) (SweepResult :type Hit%20Result%20Structure%20%28by%20ref%29))
  (if (Utilities|Enum|Equal(Enum) (Variables|Default|GetWho's%20it%20for?) "Mage")
    (bind _asmage (Utilities|Casting|CastToMage OtherActor))
    (Default|MageatDestination _asmage)
    (elif (Utilities|Enum|Equal(Enum) (Variables|Default|GetWho's%20it%20for?) "Doc")
      (bind _asdoc (Utilities|Casting|CastToDoc OtherActor))
      (Default|DocatDestination _asdoc)
      (else
        (bind _asthe_player (Utilities|Casting|CastToThePlayer OtherActor))
        (Default|CheckforFinish _asthe_player)))))

(fn ConstructionScript)