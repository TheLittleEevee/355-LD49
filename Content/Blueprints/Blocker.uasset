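; Blocker is an actor, apparently an obstacle, that removes itself based on what item the player has.
; Every tick it casts the player pawn to ThePlayer and branches on its BlockingUntilWhat string.
; The Book and Instrument cases destroy the actor once the matching flag in the player's Details is set.
; The Blanket case destroys it without checking any item flag.
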(event EventTick
  (params (DeltaSeconds :type Float%20%28single-precision%29))
  (bind _asthe_player (Utilities|Casting|CastToThePlayer (Game|Player|GetPlayerPawn 0)))
  (if (Utilities|Enum|Equal(Enum) (Variables|Default|GetBlocking%20until%20what?) "Book")
    (if (.hasbook (Variables|/Game/Blueprints/PlayerAndGame/ThePlayer.ThePlayer_C|GetDetails _asthe_player))
      (Actor|DestroyActor))
    (elif (Utilities|Enum|Equal(Enum) (Variables|Default|GetBlocking%20until%20what?) "Instrument")
      (if (.hasinstrument (Variables|/Game/Blueprints/PlayerAndGame/ThePlayer.ThePlayer_C|GetDetails _asthe_player))
        (Actor|DestroyActor))
      (elif (Utilities|Enum|Equal(Enum) (Variables|Default|GetBlocking%20until%20what?) "Blanket")
        (Actor|DestroyActor)))))

(fn ConstructionScript)