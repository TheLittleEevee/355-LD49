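; Player controller that owns the in-game HUD and pause menu and handles returning to the title screen.
; On BeginPlay it creates the HUD, which UpdateTheHUD refreshes from the player details stored in the game instance.
; The Pause input toggles game pause, switching input mode and cursor and creating or removing a pause widget whose Resume and Exit events are bound.
; Exiting unpauses, opens the title level and resets the stored player details.
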(event Custom|Update%20the%20HUD
  (bind _the_hud (Variables|Default|GetThe%20HUD))
  (Utilities|IsValid _the_hud
    (:Is%20Valid
      ;[1 1 1] TheHUD.UpdateHUD()
      (bind _output_get (Variables|Default|SetThe%20Player%20Details (Variables|/Game/Blueprints/MyGameInstance.MyGameInstance_C|GetPlayer%20Details (Variables|Default|GetThe%20Game%20Instance))))
      (Default|UpdateHUD _the_hud _output_get))))

(event Custom|Pause%20the%20Game
  (bind _self self)
  (Game|SetGamePaused true)
  ;[1 1 1] Input Mode to GAME / UI
  (Input|SetInputModeGameandUI _self 0 "DoNotLock" true)
  (Variables|Default|SetbShowMouseCursor _self true)
  ;[1 1 1] Add Pause Widget
  (bind _returnvalue (UserInterface|CreateWidget "/Game/Blueprints/GUI/PauseMenu.PauseMenu_C"))
  (bind _output_get (Variables|Default|SetThe%20Pause%20Menu _returnvalue))
  (UserInterface|Viewport|AddtoPlayerScreen _output_get)
  (EventDispatchers|BindEventtoClickedonResumeButton (Variables|Default|GetThe%20Pause%20Menu) (delegate Custom|Unpause%20the%20Game))
  (EventDispatchers|BindEventtoClickedonExitButton (Variables|Default|GetThe%20Pause%20Menu) (delegate Custom|Exit%20to%20Title)))

(event Custom|Unpause%20the%20Game
  (bind _self self)
  (Game|SetGamePaused false)
  ;[1 1 1] Input mode to GAME
  (Input|SetInputModeGameOnly _self)
  (Variables|Default|SetbShowMouseCursor _self false)
  ;[1 1 1] Remove Pause Widget
  (Utilities|IsValid (Variables|Default|GetThe%20Pause%20Menu)
    (:Is%20Valid
      (EventDispatchers|UnbindallEventsfromClickedonResumeButton (Variables|Default|GetThe%20Pause%20Menu))
      (EventDispatchers|UnbindallEventsfromClickedonExitButton (Variables|Default|GetThe%20Pause%20Menu))
      (Widget|RemovefromParent (Variables|Default|GetThe%20Pause%20Menu))
      (Variables|Default|SetThe%20Pause%20Menu 0))))

(event Custom|Exit%20to%20Title
  (CallFunction|UnpausetheGame)
  (Game|OpenLevel(byName) "TitleScreen")
  (Variables|/Game/Blueprints/MyGameInstance.MyGameInstance_C|SetPlayer%20Details (Variables|Default|GetThe%20Game%20Instance) (Utilities|Struct|MakePlayerDetails 1.0 false false false 0 false false)))

(event EventBeginPlay
  (bind _asmy_game_instance (Utilities|Casting|CastToMyGameInstance (Game|GetGameInstance)))
  (Variables|Default|SetThe%20Game%20Instance _asmy_game_instance)
  (bind _returnvalue (UserInterface|CreateWidget "/Game/Blueprints/GUI/HUD.HUD_C"))
  (bind _output_get (Variables|Default|SetThe%20HUD _returnvalue))
  (UserInterface|Viewport|AddtoViewport _output_get 0)
  (CallFunction|UpdatetheHUD))

(event EventDestroyed
  (bind _the_hud (Variables|Default|GetThe%20HUD))
  (Utilities|IsValid _the_hud
    (:Is%20Valid
      (Widget|RemovefromParent _the_hud))))

(event Input|ActionEvents|InputActionPause
  (params (Key :type Key%20Structure :default "None"))
  (:Pressed
    (if (Game|IsGamePaused)
      (CallFunction|UnpausetheGame)
      (else
        (CallFunction|PausetheGame)))))

(fn ConstructionScript)