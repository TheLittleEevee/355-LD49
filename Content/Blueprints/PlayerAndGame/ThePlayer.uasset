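; Player character for a Paper2D quest game, tracking progress in a Details struct loaded from MyGameInstance and draining sanity every tick.
; Movement inputs set facing and pick walk flipbooks by the collected book, instrument and blanket.
; Interact line-traces in the facing direction to open a paused NPC dialogue, or closes the open one.
; Quest events update Details, and CheckforFinish loads FinishGame and resets progress once all three items are held.
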(event Custom|Finished%20Helping
  (params (Helped%20Who? :type String))
  (if (Utilities|Enum|Equal(Enum) Helped%20Who? "Bard")
    (Variables|Default|SetDetails (Utilities|Struct|MakePlayerDetails (.sanity (Variables|Default|GetDetails)) (.hasblanket (Variables|Default|GetDetails)) (.hasbook (Variables|Default|GetDetails)) true (.musicsheets (Variables|Default|GetDetails)) (.talkedtoparent (Variables|Default|GetDetails)) (.childiscured (Variables|Default|GetDetails))))
    (elif (Utilities|Enum|Equal(Enum) Helped%20Who? "Librarian")
      (Variables|Default|SetDetails (Utilities|Struct|MakePlayerDetails (.sanity (Variables|Default|GetDetails)) (.hasblanket (Variables|Default|GetDetails)) true (.hasinstrument (Variables|Default|GetDetails)) (.musicsheets (Variables|Default|GetDetails)) (.talkedtoparent (Variables|Default|GetDetails)) (.childiscured (Variables|Default|GetDetails))))
      (elif (Utilities|Enum|Equal(Enum) Helped%20Who? "Child")
        (Variables|Default|SetDetails (Utilities|Struct|MakePlayerDetails (.sanity (Variables|Default|GetDetails)) true (.hasbook (Variables|Default|GetDetails)) (.hasinstrument (Variables|Default|GetDetails)) (.musicsheets (Variables|Default|GetDetails)) (.talkedtoparent (Variables|Default|GetDetails)) (.childiscured (Variables|Default|GetDetails))))))))

(event Custom|Talked%20to%20Parent
  (Variables|Default|SetDetails (Utilities|Struct|MakePlayerDetails (.sanity (Variables|Default|GetDetails)) (.hasblanket (Variables|Default|GetDetails)) (.hasbook (Variables|Default|GetDetails)) (.hasinstrument (Variables|Default|GetDetails)) (.musicsheets (Variables|Default|GetDetails)) true (.childiscured (Variables|Default|GetDetails)))))

(event Custom|Child%20is%20Better
  (Variables|Default|SetDetails (Utilities|Struct|MakePlayerDetails (.sanity (Variables|Default|GetDetails)) (.hasblanket (Variables|Default|GetDetails)) (.hasbook (Variables|Default|GetDetails)) (.hasinstrument (Variables|Default|GetDetails)) (.musicsheets (Variables|Default|GetDetails)) (.talkedtoparent (Variables|Default|GetDetails)) true)))

(event Custom|Check%20for%20Finish
  (if (Math|Boolean|ANDBoolean (.hasblanket (Variables|Default|GetDetails)) (.hasbook (Variables|Default|GetDetails)) (.hasinstrument (Variables|Default|GetDetails)))
    (Input|SetInputModeGameOnly (Game|GetPlayerController 0))
    (Game|OpenLevel(byName) "FinishGame")
    (Variables|Default|SetDetails (Utilities|Struct|MakePlayerDetails 1.0 false false false 0 false false))
    (Variables|/Game/Blueprints/MyGameInstance.MyGameInstance_C|SetPlayer%20Details (Variables|Default|GetMy%20Game%20Instance) (Utilities|Struct|MakePlayerDetails 1.0 false false false 0 false false))))

(event EventBeginPlay
  (bind _asmy_game_instance (Utilities|Casting|CastToMyGameInstance (Game|GetGameInstance)))
  (bind _output_get (Variables|Default|SetMy%20Game%20Instance _asmy_game_instance))
  (Variables|Default|SetDetails (Variables|/Game/Blueprints/MyGameInstance.MyGameInstance_C|GetPlayer%20Details _output_get)))

(event EventTick
  (params (DeltaSeconds :type Float%20%28single-precision%29))
  (Default|SanityChanges (Variables|Default|GetMy%20Game%20Instance) -0.0001))

(event Input|ActionEvents|InputActionInteract
  (params (Key :type Key%20Structure :default "None"))
  (bind _facing (Variables|Default|GetFacing))
  (bind _paperflipbook (Variables|Default|GetPaperFlipbook))
  (bind _returnvalue (Transformation|GetWorldLocation _paperflipbook))
  (:Pressed
    (if (Game|IsGamePaused)
      ;[1 1 1] Leaving Dialogue
      (Utilities|IsValid (Variables|Default|GetDialogueWindow)
        (:Is%20Valid
          (Game|SetGamePaused false)
          (Input|SetInputModeGameOnly (Game|GetPlayerController 0))
          (Utilities|IsValid (Variables|Default|GetDialogueWindow)
            (:Is%20Valid
              (Widget|RemovefromParent (Variables|Default|GetDialogueWindow))
              (Variables|Default|SetDialogueWindow 0)))))
      (else
        ;[1 1 1] Directional Interact (for Dialogue)
        (if (Utilities|Enum|Equal(Enum) _facing "R")
          (Variables|Default|SetInteracting%20Vector "65.000000,65.000000, 0")
          (elif (Utilities|Enum|Equal(Enum) _facing "B")
            (Variables|Default|SetInteracting%20Vector "-65.000000,65.000000, 0")
            (elif (Utilities|Enum|Equal(Enum) _facing "L")
              (Variables|Default|SetInteracting%20Vector "-65.000000,-65.000000, 0")
              (else
                (Variables|Default|SetInteracting%20Vector "65.000000,-65.000000, 0")))))
        (bind (_outhit _returnvalue_2) (Collision|LineTraceByChannel _returnvalue (+ _returnvalue (Variables|Default|GetInteracting%20Vector)) "TraceTypeQuery1" false 0 "ForDuration" true "(R=1.000000,G=0.000000,B=0.000000,A=1.000000)" "(R=0.000000,G=1.000000,B=0.000000,A=1.000000)" 0.0))
        (if _returnvalue_2
          (if (Utilities|DoesObjectImplementInterface (.HitActor (Collision|BreakHitResult _outhit)) "/Game/Blueprints/Interfaces/PlayerCanInteract.PlayerCanInteract_C")
            (bind _asnpcs (Utilities|Casting|CastToNPCs (.HitActor (Collision|BreakHitResult _outhit))))
            (Game|SetGamePaused true)
            (Input|SetInputModeGameandUI (Game|GetPlayerController 0) 0 "DoNotLock" false)
            (bind _returnvalue_3 (UserInterface|CreateWidget "/Game/Blueprints/GUI/Dialogue.Dialogue_C"))
            (Default|GiveTextInfo _asnpcs _returnvalue_3 self)
            (bind _output_get (Variables|Default|SetDialogueWindow _returnvalue_3))
            (UserInterface|Viewport|AddtoPlayerScreen _output_get)))))))

(event Input|AxisEvents|InputAxisMoveForward
  (params (AxisValue :type Float%20%28single-precision%29))
  (bind _returnvalue (Transformation|GetActorForwardVector))
  (bind _details (Variables|Default|GetDetails))
  (bind _right_axis (Variables|Default|GetRight%20Axis))
  (bind _paperflipbook (Variables|Default|GetPaperFlipbook))
  (bind _returnvalue_2 (== _right_axis 0.0))
  ;[1 1 1] Move
  (Variables|Default|SetForward%20Axis AxisValue)
  (Pawn|Input|AddMovementInput (Math|Vector|MakeVector (.x _returnvalue) (.y _returnvalue) 0.0) (/ AxisValue 1.75) false)
  (if (> AxisValue 0.0)
    (Variables|Default|SetFacing "F")
    (if _returnvalue_2
      (if (.hasbook _details)
        (if (.hasinstrument _details)
          (if (.hasblanket _details)
            (Sprite|SetFlipbook _paperflipbook "/Game/Art/Assets/Characters/catboywalk/blanket/back/main_sprite_blanket_back.main_sprite_blanket_back")
            (else
              (Sprite|SetFlipbook _paperflipbook "/Game/Art/Assets/Characters/catboywalk/Lute/back/mail_sprite_lute_back.mail_sprite_lute_back")))
          (else
            (Sprite|SetFlipbook _paperflipbook "/Game/Art/Assets/Characters/catboywalk/Book/back/main_sprite_book_back_walk.main_sprite_book_back_walk")))
        (else
          (Sprite|SetFlipbook _paperflipbook "/Game/Art/Assets/Characters/catboywalk/No_Items/back/walk_back_sprite.walk_back_sprite"))))
    (elif (< AxisValue 0.0)
      (Variables|Default|SetFacing "B")
      (if _returnvalue_2
        (if (.hasbook _details)
          (if (.hasinstrument _details)
            (if (.hasblanket _details)
              (Sprite|SetFlipbook _paperflipbook "/Game/Art/Assets/Characters/catboywalk/blanket/front/NewPaperFlipbook.NewPaperFlipbook")
              (else
                (Sprite|SetFlipbook _paperflipbook "/Game/Art/Assets/Characters/catboywalk/Lute/front/main_sprite_lute_front_walk.main_sprite_lute_front_walk")))
            (else
              (Sprite|SetFlipbook _paperflipbook "/Game/Art/Assets/Characters/catboywalk/Book/front/main_sprite_book_front_walk.main_sprite_book_front_walk")))
          (else
            (Sprite|SetFlipbook _paperflipbook "/Game/Art/Assets/Characters/catboywalk/No_Items/front/walk_back_sprite.walk_back_sprite")))))))

(event Input|AxisEvents|InputAxisMoveRight
  (params (AxisValue :type Float%20%28single-precision%29))
  (bind _details (Variables|Default|GetDetails))
  (bind _paperflipbook (Variables|Default|GetPaperFlipbook))
  ;[1 1 1] Move
  (Variables|Default|SetRight%20Axis AxisValue)
  (Pawn|Input|AddMovementInput (Transformation|GetActorRightVector) (/ AxisValue 1.75) false)
  (if (> AxisValue 0.0)
    (Variables|Default|SetFacing "R")
    (if (.hasbook _details)
      (if (.hasinstrument _details)
        (if (.hasblanket _details)
          (Sprite|SetFlipbook _paperflipbook "/Game/Art/Assets/Characters/catboywalk/blanket/right/main_sprite_blanket_right_walk.main_sprite_blanket_right_walk")
          (else
            (Sprite|SetFlipbook _paperflipbook "/Game/Art/Assets/Characters/catboywalk/Lute/right/main_sprite_lute_right_walk.main_sprite_lute_right_walk")))
        (else
          (Sprite|SetFlipbook _paperflipbook "/Game/Art/Assets/Characters/catboywalk/Book/right/main_sprite_book_right_walk.main_sprite_book_right_walk")))
      (else
        (Sprite|SetFlipbook _paperflipbook "/Game/Art/Assets/Characters/catboywalk/No_Items/right/walk_right_sprite.walk_right_sprite")))
    (elif (< AxisValue 0.0)
      (Variables|Default|SetFacing "L")
      (if (.hasbook _details)
        (if (.hasinstrument _details)
          (if (.hasblanket _details)
            (Sprite|SetFlipbook _paperflipbook "/Game/Art/Assets/Characters/catboywalk/blanket/left/main_sprite_blanket_left_walk.main_sprite_blanket_left_walk")
            (else
              (Sprite|SetFlipbook _paperflipbook "/Game/Art/Assets/Characters/catboywalk/Lute/left/main_sprite_lute_left_walk.main_sprite_lute_left_walk")))
          (else
            (Sprite|SetFlipbook _paperflipbook "/Game/Art/Assets/Characters/catboywalk/Book/left/main_sprite_book_left_walk.main_sprite_book_left_walk")))
        (else
          (Sprite|SetFlipbook _paperflipbook "/Game/Art/Assets/Characters/catboywalk/No_Items/left/walk_left_sprite.walk_left_sprite"))))))

(fn ConstructionScript)