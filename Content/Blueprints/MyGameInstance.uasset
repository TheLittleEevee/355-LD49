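; Game instance that stores the player's persistent details: sanity, item flags, music sheet count and quest progress for a parent and child.
; SanityChanges applies a clamped sanity delta, then refreshes the HUD through MyPlayerController.
; At zero sanity it switches to game-only input, opens the GameOver level and resets the details to defaults.
; MoreMusicSheets increments the collected sheet count.
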(fn SanityChanges
  (params (Change%20in%20Sanity :type Float%20%28single-precision%29))
  (Variables|Default|SetPlayer%20Details (Utilities|Struct|MakePlayerDetails (Math|Float|Clamp(Float) (+ (.sanity (Variables|Default|GetPlayer%20Details)) Change%20in%20Sanity)) (.hasblanket (Variables|Default|GetPlayer%20Details)) (.hasbook (Variables|Default|GetPlayer%20Details)) (.hasinstrument (Variables|Default|GetPlayer%20Details)) (.musicsheets (Variables|Default|GetPlayer%20Details)) (.talkedtoparent (Variables|Default|GetPlayer%20Details)) (.childiscured (Variables|Default|GetPlayer%20Details))))
  (bind _asmy_player_controller (Utilities|Casting|CastToMyPlayerController (Game|GetPlayerController 0)))
  (Default|UpdatetheHUD _asmy_player_controller)
  (if (<= (.sanity (Variables|Default|GetPlayer%20Details)) 0.0)
    (Input|SetInputModeGameOnly (Game|GetPlayerController 0))
    (Game|OpenLevel(byName) "GameOver")
    (Variables|Default|SetPlayer%20Details (Utilities|Struct|MakePlayerDetails 1.0 false false false 0 false false))))

(fn MoreMusicSheets
  (Variables|Default|SetPlayer%20Details (Utilities|Struct|MakePlayerDetails (.sanity (Variables|Default|GetPlayer%20Details)) (.hasblanket (Variables|Default|GetPlayer%20Details)) (.hasbook (Variables|Default|GetPlayer%20Details)) (.hasinstrument (Variables|Default|GetPlayer%20Details)) (+ (.musicsheets (Variables|Default|GetPlayer%20Details)) 1) (.talkedtoparent (Variables|Default|GetPlayer%20Details)) (.childiscured (Variables|Default|GetPlayer%20Details)))))