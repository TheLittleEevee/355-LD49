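; Pickup item actor that acts as either a music sheet or a sanity-affecting food.
; On BeginPlay it picks its paper sprite from the MusicSheet flag or, for food, from the SanityEffect value (mac and cheese or cookie).
; When ThePlayer overlaps its box, it reports to MyGameInstance through MoreMusicSheets or SanityChanges, then destroys itself.
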(event OnComponentBeginOverlap(Box)
  (params (OverlappedComponent :type Primitive%20Component%20Object%20Reference) (OtherActor :type Actor%20Object%20Reference) (OtherComp :type Primitive%20Component%20Object%20Reference) (OtherBodyIndex :type Integer) (bFromSweep :type Boolean) (SweepResult :type Hit%20Result%20Structure%20%28by%20ref%29))
  (Utilities|Casting|CastToThePlayer OtherActor)
  (bind _asmy_game_instance (Utilities|Casting|CastToMyGameInstance (Game|GetGameInstance)))
  (Variables|Default|SetPlayer%20Detail (Variables|/Game/Blueprints/MyGameInstance.MyGameInstance_C|GetPlayer%20Details _asmy_game_instance))
  (if (Variables|Default|GetMusic%20Sheet?)
    (Default|MoreMusicSheets _asmy_game_instance)
    (else
      (Default|SanityChanges _asmy_game_instance (Variables|Default|GetSanity%20Effect))))
  (Actor|DestroyActor))

(event EventBeginPlay
  (if (Variables|Default|GetMusic%20Sheet?)
    (Rendering|Components|Sprite|SetSprite (Variables|Default|GetPaperSprite) "/Game/Art/Assets/MusicSheet_MusicSheet_0_Sprite.MusicSheet_MusicSheet_0_Sprite")
    (elif (== (Variables|Default|GetSanity%20Effect) 1.0)
      (Rendering|Components|Sprite|SetSprite (Variables|Default|GetPaperSprite) "/Game/Art/Assets/MacNCheese_Food_2_0_Sprite.MacNCheese_Food_2_0_Sprite")
      (elif (== (Variables|Default|GetSanity%20Effect) 0.5)
        (Rendering|Components|Sprite|SetSprite (Variables|Default|GetPaperSprite) "/Game/Art/Assets/Cookie_Food_0_Sprite.Cookie_Food_0_Sprite")))))

(fn ConstructionScript)